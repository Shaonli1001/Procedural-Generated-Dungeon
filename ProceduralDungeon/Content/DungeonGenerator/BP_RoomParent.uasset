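; BP_RoomParent is the parent room actor for a dungeon generator, able to open paths toward the rooms it connects to.
; On BeginPlay it stores its world X/Y location as Coordinates.
; Createpaths compares each RoomConnection entry's Coordinates with its own and destroys the Top, Bottom, Right or Left component facing that neighbor.
; X differences take priority, so each connection resolves to a single side.
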(event Custom|Create%20paths
  (bind _result (Utilities|Set|ToArray (Variables|Default|GetRoomConnection)))
  (for _array_element _result
    (if (!= (.x (Variables|BP_RoomParent_C|GetCoordinates _array_element)) (.x (Variables|Default|GetCoordinates)))
      (if (> (.x (Variables|BP_RoomParent_C|GetCoordinates _array_element)) (.x (Variables|Default|GetCoordinates)))
        (Components|DestroyComponent (Variables|Default|GetTop))
        (else
          (Components|DestroyComponent (Variables|Default|GetBottom))))
      (elif (> (.y (Variables|BP_RoomParent_C|GetCoordinates _array_element)) (.y (Variables|Default|GetCoordinates)))
        (Components|DestroyComponent (Variables|Default|GetRight))
        (else
          (Components|DestroyComponent (Variables|Default|GetLeft)))))))

(event EventBeginPlay
  (bind _returnvalue (Transformation|GetActorLocation))
  (Variables|Default|SetCoordinates (Math|Vector2D|MakeVector2D (.x _returnvalue) (.y _returnvalue))))

(fn ConstructionScript)